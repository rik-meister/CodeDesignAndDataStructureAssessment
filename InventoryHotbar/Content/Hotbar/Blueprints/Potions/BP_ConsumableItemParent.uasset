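; Parent Blueprint for consumable item pickups such as potions, which the player collects into the inventory by walking into them.
; On BeginPlay it looks up its item data in DT_InventoryItemData using its item ID.
; When a first-person character overlaps the sphere, it calls AddItem on that character's inventory component.
; On success it shows a HUD notification with the item data and amount, then destroys itself.
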(event `self.ReceiveBeginPlay`
  (`self.InitializeItemDataStruct`))

(event `self.Sphere1.OnComponentBeginOverlap`
  (params (OverlappedComponent :type "PrimitiveComponent Object Reference") (OtherActor :type "Actor Object Reference") (OtherComp :type "PrimitiveComponent Object Reference") (OtherBodyIndex :type Integer) (bFromSweep :type Boolean) (SweepResult :type "HitResult Structure (by ref)"))
  (bind _asbp_first_person_character (cast `/Game/FirstPerson/Blueprints/BP_FirstPersonCharacter` OtherActor))
  (bind _success_ (`/Game/Hotbar/Inventory/BPAC_InventoryComponent.AddItem` (`/Game/FirstPerson/Blueprints/BP_FirstPersonCharacter.BPAC_InventoryComponent` _asbp_first_person_character) (`self.ConsumableItem_ID`) (`self.ConsumableItem_Amount`)))
  (if _success_
    (`/Game/Hotbar/UI/WBP_UserHUD.AddItemNotification` (`/Game/FirstPerson/Blueprints/BP_FirstPersonCharacter.PlayerHUD_Ref` _asbp_first_person_character) (`self.ConsumableItem_Data`) (`self.ConsumableItem_Amount`))
    (`self.K2_DestroyActor`)))

(fn `InitializeItemDataStruct`
  (bind _returnvalue (`|GetDataTableRow` "/Game/Hotbar/DataTables/DT_InventoryItemData.DT_InventoryItemData" (`KismetStringLibrary.Conv_StringToName` (`self.ConsumableItem_ID`)))
    (:`then`
      (set `self.ConsumableItem_Data` _returnvalue))))

(fn `UserConstructionScript`)