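; Inventory component that manages a fixed-size hotbar of item data slots and equips the selected item on its owner.
; Scrolling wraps through the numbered slots, with slot 0 meaning nothing equipped, and added items fill the first free slot and are equipped immediately.
; Equipping adds the item's component class to BP_FirstPersonCharacter, tagged "Item" so unequip can pass it to the owner through BI_BT_Inventory.
; Dispatchers announce initialization and equip changes.
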(event `self.ReceiveBeginPlay`
  (`self.SetupInventory`))

(fn `AddItem`
  (params (NewItemData :type "/Game/Hotbar/DataAssets/PDA_BT_Item Object Reference"))
  (locals (FreeItemSlotIndex :type Integer))
  (bind _itemslotlist (`self.ItemSlotList`))
  (bind _freeitemslotindex (`local.FreeItemSlotIndex`))
  (bind _returnvalue (+ _freeitemslotindex 1))
  (for (_array_element _array_index) _itemslotlist
    (`/Engine/EditorBlueprintResources/StandardMacros.IsValid` _array_element
      (:`Is Not Valid`
        (set `local.FreeItemSlotIndex` _array_index)
        (break))))
  (`KismetArrayLibrary.Array_Set` _itemslotlist _freeitemslotindex NewItemData)
  (set `self.ItemSlotSelectedNumber` _returnvalue)
  (`self.EquipItemSlot` _returnvalue))

(fn `EquipItemSlot`
  (params (NewItemSlotNumber :type Integer))
  (`self.UnequipItem`)
  (if (not (== NewItemSlotNumber 0))
    (bind _itemdata (`self.GetItemDataFromItemSlotNumber` NewItemSlotNumber))
    (`/Engine/EditorBlueprintResources/StandardMacros.IsValid` _itemdata
      (:`Is Valid`
        (set `self.ItemSlotSelectedData` _itemdata)
        (bind _asbp_first_person_character (cast `/Game/FirstPerson/Blueprints/BP_FirstPersonCharacter` (`self.GetOwner`)))
        (bind _returnvalue (`|AddComponentByClass` :`self` _asbp_first_person_character :`Class` (`/Game/Hotbar/DataAssets/PDA_BT_Item.Item` (`self.ItemSlotSelectedData`))))
        (set `ActorComponent.ComponentTags` (`|MakeArray` "Item" :!type "Name") _returnvalue)
        (set `self.ItemSelectedActor` _returnvalue)
        (`self.OnItemEquipped` (`self.ItemSlotSelectedNumber`) (`self.ItemSlotSelectedData`))))))

(fn `GetInventory`
  (returns (ItemSlotList :type "Array of /Game/Hotbar/DataAssets/PDA_BT_Item Object Reference") (InventorySize :type Integer))
  (return (`self.ItemSlotList`) (`self.InventorySize`)))

(fn `GetItemDataFromItemSlotNumber`
  (params (ItemSlotNumber :type Integer))
  (returns (ItemData :type "/Game/Hotbar/DataAssets/PDA_BT_Item Object Reference"))
  (return (`|GetArrayItem` (`self.ItemSlotList`) (`self.GetItemSlotIndexFromItemSlotNumber` ItemSlotNumber))))

(fn `GetItemSlotIndexFromItemSlotNumber`
  (params (ItemSlotNumber :type Integer))
  (returns (ItemSlotIndex :type Integer))
  (return (- ItemSlotNumber 1)))

(fn `ScrollWeaponSelection`
  (params (Increment :type Integer))
  (bind _output_get (set `self.ItemSlotSelectedNumber` (+ (`self.ItemSlotSelectedNumber`) Increment)))
  ;[1 1 1] Below Min
  (if (<= _output_get -1)
    ;[1 1 1] Reset to MAX Slot
    (set `self.ItemSlotSelectedNumber` (`self.InventorySize`))
    (elif (>= (`self.ItemSlotSelectedNumber`) (+ (`self.InventorySize`) 1))
      ;[1 1 1] Reset to MIN Slot
      (set `self.ItemSlotSelectedNumber` 0)))
  (`self.EquipItemSlot` (`self.ItemSlotSelectedNumber`)))

(fn `SelectNextWeapon`
  (`self.ScrollWeaponSelection` 1))

(fn `SelectPreviousWeapon`
  (`self.ScrollWeaponSelection` -1))

(fn `SetupInventory`
  (if (== (`KismetArrayLibrary.Array_Length` (`self.ItemSlotList`)) 0)
    (for _ (range 1 (+ (`self.InventorySize`) 1))
      (`KismetArrayLibrary.Array_Add` (`self.ItemSlotList`))))
  (`self.OnInventoryInitialized` (`self.ItemSlotList`)))

(fn `UnequipItem`
  (bind _returnvalue (`self.GetOwner`))
  (if (`KismetSystemLibrary.DoesImplementInterface` _returnvalue "/Game/Hotbar/Interfaces/BI_BT_Inventory.BI_BT_Inventory_C")
    (message `/Game/Hotbar/Interfaces/BI_BT_Inventory.Unequip` _returnvalue (`Actor.FindComponentByTag` _returnvalue "/Script/Engine.ActorComponent" "Item"))
    (`self.OnItemEquipped` 0 (`self.ItemSlotSelectedData`))))